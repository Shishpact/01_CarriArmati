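; Player-controllable tank Blueprint that maps input to driving, firing and camera rotation.
; Forward and lateral axes send intentions to the Movimento component, initialized on BeginPlay with both tracks, while two separate axes can drive each track directly.
; BeginPlay also registers Barrel and Turret via setters, and the Fuoco action calls the Aiming component's SpawnOggetto.
; Camera orbit splits yaw onto a Scene component and pitch onto the SpringArm.
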(event EventBeginPlay
  (Class|TankCPP|SetCannone (Variables|Default|GetBarrel))
  (Class|TankCPP|SetTorre (Variables|Default|GetTurret))
  (Class|Movimento|Inizialize (Variables|Default|GetMovimento) (Variables|Default|GetTrackDX) (Variables|Default|GetTrackSX)))

(event Collision|EventActorBeginOverlap
  (params (OtherActor :type Actor%20Object%20Reference)))

(event EventTick
  (params (DeltaSeconds :type Float%20%28single-precision%29)))

(event Input|ActionEvents|InputActionFuoco
  (params (Key :type Key%20Structure))
  (:Pressed
    (Class|AimingCPP|SpawnOggetto (Variables|Default|GetAiming))))

(event Input|AxisEvents|InputAxisMoveForward
  (params (AxisValue :type Float%20%28single-precision%29))
  (Class|Movimento|IntenzioneAvanti (Variables|Default|GetMovimento) AxisValue))

(event Input|AxisEvents|InputAxisMoveRight
  (params (AxisValue :type Float%20%28single-precision%29))
  (Class|Movimento|IntenzioneLaterale (Variables|Default|GetMovimento) AxisValue))

(event Input|AxisEvents|InputAxisCingoloDF
  (params (AxisValue :type Float%20%28single-precision%29))
  (Class|MeshCingolo|RichiestaMovimento (Variables|Default|GetTrackDX) AxisValue))

(event Input|AxisEvents|InputAxisCingoloSF
  (params (AxisValue :type Float%20%28single-precision%29))
  (Class|MeshCingolo|RichiestaMovimento (Variables|Default|GetTrackSX) AxisValue))

(event Input|AxisEvents|InputAxisLevatura
  (params (AxisValue :type Float%20%28single-precision%29))
  (Transformation|AddLocalRotation (Variables|Default|GetSpringArm) (Math|Rotator|MakeRotator 0.0 AxisValue 0.0) false false))

(event Input|AxisEvents|InputAxisAzimuth
  (params (AxisValue :type Float%20%28single-precision%29))
  (Transformation|AddLocalRotation (Variables|Default|GetScene) (Math|Rotator|MakeRotator 0.0 0.0 AxisValue) false false))

(fn ConstructionScript)